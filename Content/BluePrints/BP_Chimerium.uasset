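; BP_Chimerium is a scannable ore actor that signals detection when something overlaps its collider.
; Overlap runs a check that plays an attenuated OreDetected sound for scan collision actors, identified by display-name substring, while custom depth stencil briefly marks the sphere.
; A Tick countdown periodically restores the polystyrene material; the scan-glow material change is never run.
; BeginPlay fills a spawn location array, unused here.
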(event OnComponentBeginOverlap(Collider)
  (params (OverlappedComponent :type Primitive%20Component%20Object%20Reference) (OtherActor :type Actor%20Object%20Reference) (OtherComp :type Primitive%20Component%20Object%20Reference) (OtherBodyIndex :type Integer) (bFromSweep :type Boolean) (SweepResult :type Hit%20Result%20Structure%20%28by%20ref%29))
  (bind _sphere (Variables|Default|GetSphere))
  (|Sound&CheckingLogic_2 OtherActor OtherActor)
  (Rendering|SetCustomDepthStencilValue _sphere 1)
  (Utilities|FlowControl|Delay 3.0)
  (Rendering|SetCustomDepthStencilValue _sphere 0))

(event EventTick
  (params (DeltaSeconds :type Float%20%28single-precision%29))
  ;[1 1 1] Material Change Cooldown
  (Variables|Default|SetRemainingScanTime (- (Variables|Default|GetRemainingScanTime) DeltaSeconds))
  (if (< (Variables|Default|GetRemainingScanTime) 0.0)
    (Rendering|Material|SetMaterial (Variables|Default|GetSphere) 0 "/Game/Megascans/Surfaces/Polystyrene_rfya3fp0/MI_Polystyrene_rfya3fp0_2K.MI_Polystyrene_rfya3fp0_2K")
    (Variables|Default|SetRemainingScanTime 3.0)))

(event EventBeginPlay
  (Variables|Default|SetChimeriumSpawnLocations (Utilities|Array|MakeArray (Variables|Default|GetSpawnOne) (Variables|Default|GetSpawnOne1) (Variables|Default|GetSpawnOne2) (Variables|Default|GetSpawnOne3) (Variables|Default|GetSpawnOne4) (Variables|Default|GetSpawnOne5))))

(fn ConstructionScript
  (|CallParentFunction))