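; BP_ExplodingPlant is a cactus hazard that reacts to proximity and explodes.
; WarningRegion switches the skeletal mesh between looping flinch and idle animations as the first-person character enters and leaves.
; Any actor with a BP_Health component entering ExplodeRegion triggers the explode animation and, after a short delay, destruction of the plant.
; Damage always goes to player character 0, regardless of who triggered it or current distance.
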(event OnComponentBeginOverlap(WarningRegion)
  (params (OverlappedComponent :type Primitive%20Component%20Object%20Reference) (OtherActor :type Actor%20Object%20Reference) (OtherComp :type Primitive%20Component%20Object%20Reference) (OtherBodyIndex :type Integer) (bFromSweep :type Boolean) (SweepResult :type Hit%20Result%20Structure%20%28by%20ref%29))
  (Utilities|Casting|CastToBP_FirstPersonCharacter OtherActor)
  (if true
    (Components|Animation|PlayAnimation (Variables|Default|GetSkeletalMesh) "/Game/ImportedAssets/ExplodingPlant/Exploding_Barrel_Cactus_Anim_xen_barrel_cactus_qc_skeleton_Flinch.Exploding_Barrel_Cactus_Anim_xen_barrel_cactus_qc_skeleton_Flinch" true)))

(event OnComponentBeginOverlap(ExplodeRegion)
  (params (OverlappedComponent :type Primitive%20Component%20Object%20Reference) (OtherActor :type Actor%20Object%20Reference) (OtherComp :type Primitive%20Component%20Object%20Reference) (OtherBodyIndex :type Integer) (bFromSweep :type Boolean) (SweepResult :type Hit%20Result%20Structure%20%28by%20ref%29))
  (Utilities|IsValid (Actor|GetComponentbyClass OtherActor "/Game/BluePrints/BP_Health.BP_Health_C")
    (:Is%20Valid
      (Components|Animation|PlayAnimation (Variables|Default|GetSkeletalMesh) "/Game/ImportedAssets/ExplodingPlant/Exploding_Barrel_Cactus_Anim_xen_barrel_cactus_qc_skeleton_explode.Exploding_Barrel_Cactus_Anim_xen_barrel_cactus_qc_skeleton_explode" true)
      (Utilities|FlowControl|Delay 1.0)
      (Game|Damage|ApplyDamage (Game|GetPlayerCharacter 0) (Variables|Default|GetDamage) 0 0)
      (Actor|DestroyActor))))

(event OnComponentEndOverlap(WarningRegion)
  (params (OverlappedComponent :type Primitive%20Component%20Object%20Reference) (OtherActor :type Actor%20Object%20Reference) (OtherComp :type Primitive%20Component%20Object%20Reference) (OtherBodyIndex :type Integer))
  (Utilities|Casting|CastToBP_FirstPersonCharacter OtherActor)
  (if true
    (Components|Animation|PlayAnimation (Variables|Default|GetSkeletalMesh) "/Game/ImportedAssets/ExplodingPlant/Exploding_Barrel_Cactus_Anim_xen_barrel_cactus_qc_skeleton_Idle.Exploding_Barrel_Cactus_Anim_xen_barrel_cactus_qc_skeleton_Idle" true)))

(fn ConstructionScript)