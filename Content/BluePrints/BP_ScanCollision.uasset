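; BP_ScanCollision is a short-lived expanding collision actor for a scan effect.
; On BeginPlay, a timeline drives the root's uniform world scale from its ScanColliderExpand curve times a fixed multiplier, then destroys the actor when finished.
; Each actor overlap adds an audio component.
; An alternative relative-scale lerp and a completion print are left disconnected, and the stored ScanScale is never read here.
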(event EventBeginPlay
  (Variables|Default|SetScan%20Scale (.scale (Transformation|GetRelativeTransform (Variables|Default|GetDefaultSceneRoot))))
  (bind _scancolliderexpand (Timeline|Timeline Play)
    (:Update
      (Transformation|SetWorldScale3D (Variables|Default|GetDefaultSceneRoot) (Math|Vector|MakeVector (* _scancolliderexpand 8e+01) (* _scancolliderexpand 8e+01) (* _scancolliderexpand 8e+01))))
    (:Finished
      (Actor|DestroyActor))))

(event Collision|EventActorBeginOverlap
  (params (OtherActor :type Actor%20Object%20Reference))
  (AddComponent|AddAudioComponent false))

(fn ConstructionScript)