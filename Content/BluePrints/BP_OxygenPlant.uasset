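; BP_OxygenPlant is an animated plant that opens when the first-person character approaches and closes when they leave.
; Begin and end overlaps on the Opening component play the open or close animation on the Plant mesh, with a sound on opening only.
; Fixed delays, rather than animation-finished events, time the switch to the looping opened or closed animation.
; The graph contains no oxygen logic.
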(event OnComponentBeginOverlap(Opening)
  (params (OverlappedComponent :type Primitive%20Component%20Object%20Reference) (OtherActor :type Actor%20Object%20Reference) (OtherComp :type Primitive%20Component%20Object%20Reference) (OtherBodyIndex :type Integer) (bFromSweep :type Boolean) (SweepResult :type Hit%20Result%20Structure%20%28by%20ref%29))
  (Utilities|Casting|CastToBP_FirstPersonCharacter OtherActor)
  (if true
    (Components|Animation|PlayAnimation (Variables|Default|GetPlant) "/Game/ImportedAssets/OxygenPlant/model_Anim_open.model_Anim_open" false)
    (Audio|PlaySoundatLocation "/Game/Audio/PlantOpenCUe.PlantOpenCUe" (Transformation|GetActorLocation) "0, 0, 0" 1.0 1.0 0.0 0 0 0 0)
    (Utilities|FlowControl|Delay 2.08)
    (Components|Animation|PlayAnimation (Variables|Default|GetPlant) "/Game/ImportedAssets/OxygenPlant/model_Anim_opened.model_Anim_opened" true)))

(event OnComponentEndOverlap(Opening)
  (params (OverlappedComponent :type Primitive%20Component%20Object%20Reference) (OtherActor :type Actor%20Object%20Reference) (OtherComp :type Primitive%20Component%20Object%20Reference) (OtherBodyIndex :type Integer))
  (Utilities|Casting|CastToBP_FirstPersonCharacter OtherActor)
  (if true
    (Components|Animation|PlayAnimation (Variables|Default|GetPlant) "/Game/ImportedAssets/OxygenPlant/model_Anim_close.model_Anim_close" false)
    (Utilities|FlowControl|Delay 3.3)
    (Components|Animation|PlayAnimation (Variables|Default|GetPlant) "/Game/ImportedAssets/OxygenPlant/model_Anim_closed.model_Anim_closed" true)))

(fn ConstructionScript)