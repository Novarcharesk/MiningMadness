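; BP_Dilithium is a dilithium ore actor that lights up when its collider is overlapped, apparently as scan feedback.
; Any overlap swaps the sphere to a glow material, while a free-running Tick countdown periodically restores the crystal material, so glow duration varies.
; BeginPlay also fills an array of five spawn points, unused here.
; The scan-collision detection sound and custom-depth stencil logic are never executed.
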(event OnComponentBeginOverlap(Collider)
  (params (OverlappedComponent :type Primitive%20Component%20Object%20Reference) (OtherActor :type Actor%20Object%20Reference) (OtherComp :type Primitive%20Component%20Object%20Reference) (OtherBodyIndex :type Integer) (bFromSweep :type Boolean) (SweepResult :type Hit%20Result%20Structure%20%28by%20ref%29))
  (Rendering|Material|SetMaterial (Variables|Default|GetSphere) 0 "/Game/MaterialsandParticles/M_ScanGlowDilithium.M_ScanGlowDilithium"))

(event EventBeginPlay
  (Variables|Default|SetBig%20Gem%20Stone%20Three%20SpawnPoint (Utilities|Array|MakeArray (Variables|Default|GetSpawnPointD1) (Variables|Default|GetSpawnPointD2) (Variables|Default|GetSpawnPointD3) (Variables|Default|GetSpawnPointD4) (Variables|Default|GetSpawnPointD5))))

(event EventTick
  (params (DeltaSeconds :type Float%20%28single-precision%29))
  ;[1 1 1] Material Change Cooldown
  (Variables|Default|SetRemainingScanTime (- (Variables|Default|GetRemainingScanTime) DeltaSeconds))
  (if (< (Variables|Default|GetRemainingScanTime) 0.0)
    (Rendering|Material|SetMaterial (Variables|Default|GetSphere) 0 "/Game/ImportedAssets/Crystals_Gems/Dilithium/Crystal_5.Crystal_5")
    (Variables|Default|SetRemainingScanTime 3.0)))

(fn ConstructionScript
  (|CallParentFunction))