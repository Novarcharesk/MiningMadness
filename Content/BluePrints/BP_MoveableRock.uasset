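; BP_MoveableRock is a rock with a detection range that maintains a CanUseDrone flag, apparently for an explosive drone.
; Begin and end overlap on ExplosiveDroneDetectionRange both set the flag by testing whether the other actor's display name contains that of BP_FirstPersonCharacter.
; Both events use the identical test, so the player leaving the range also sets the flag true.
; The file shows no movement or explosion logic.
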(event OnComponentBeginOverlap(ExplosiveDroneDetectionRange)
  (params (OverlappedComponent :type Primitive%20Component%20Object%20Reference) (OtherActor :type Actor%20Object%20Reference) (OtherComp :type Primitive%20Component%20Object%20Reference) (OtherBodyIndex :type Integer) (bFromSweep :type Boolean) (SweepResult :type Hit%20Result%20Structure%20%28by%20ref%29))
  (bind _returnvalue (Actor|GetActorOfClass "/Game/FirstPerson/Blueprints/BP_FirstPersonCharacter.BP_FirstPersonCharacter_C"))
  (Variables|Default|SetcanUseDrone (Utilities|String|Contains (Utilities|GetDisplayName OtherActor) (Utilities|GetDisplayName _returnvalue))))

(event OnComponentEndOverlap(ExplosiveDroneDetectionRange)
  (params (OverlappedComponent :type Primitive%20Component%20Object%20Reference) (OtherActor :type Actor%20Object%20Reference) (OtherComp :type Primitive%20Component%20Object%20Reference) (OtherBodyIndex :type Integer))
  (bind _returnvalue (Actor|GetActorOfClass "/Game/FirstPerson/Blueprints/BP_FirstPersonCharacter.BP_FirstPersonCharacter_C"))
  (Variables|Default|SetcanUseDrone (Utilities|String|Contains (Utilities|GetDisplayName OtherActor) (Utilities|GetDisplayName _returnvalue))))

(fn ConstructionScript)