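; Timed bomb actor that pulses with a glow, then blasts and destroys nearby BP_MoveableRock actors.
; A Delay on Tick drives a FlipFlop that alternates the glow timeline forward and backward, decrementing the countdown on each reverse.
; At expiry, a sphere trace finds rocks.
; A rock at hit index zero destroys the bomb; later ones unpause the explosion, get radial force and DestroyRock, and shorten the bomb's lifespan.
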(event EventBeginPlay
  (Class|NiagaraComponent|SetPaused (Variables|Default|GetExplosion) true)
  (Collision|SetCollisionEnabled (Variables|Default|GetBombRadius) "NoCollision"))

(event EventTick
  (params (DeltaSeconds :type Float%20%28single-precision%29))
  (Utilities|FlowControl|Delay 0.3)
  (Utilities|Time|SetTimerbyFunctionName 0 "" 0.0 false 1.0)
  (Variables|Default|SettimerStarted true)
  (Utilities|FlowControl|FlipFlop
    (:A
      (bind _newtrack_0 (Timeline|Glowing%20Bomb Play)
        (:Update
          (Rendering|Material|SetScalarParameterValueonMaterials (Variables|Default|GetBomb) "GlowSlider" _newtrack_0))))
    (:B
      (Utilities|FlowControl|Sequence
        (:then_0
          (Timeline|Glowing%20Bomb ReverseFromEnd))
        (:then_1
          (bind _output_get (Variables|Default|SetCurrentBombTimer (- (Math|Float|Clamp(Float) (Variables|Default|GetCurrentBombTimer) 0.0 1e+01) 1.0)))
          (if (<= _output_get 0.1)
            (Variables|Default|SettimerStarted false)
            (Variables|Default|SettheLocation (Transformation|GetWorldLocation (Variables|Default|GetBombRadius)))
            (bind _outhits (Collision|MultiSphereTraceForObjects (Variables|Default|GettheLocation) (Variables|Default|GettheLocation) 6e+02 (Variables|Default|GetObject%20Types) false 0 "None"))
            (for (_array_element _array_index) _outhits
              (bind _asbp_moveable_rock (Utilities|Casting|CastToBP_MoveableRock (.hitactor _array_element)))
              (if (<= _array_index 0)
                (Actor|DestroyActor)
                (Utilities|Platform|CollectGarbage)
                (else
                  (Class|NiagaraComponent|SetPaused (Variables|Default|GetExplosion) false)
                  (Class|PrimitiveComponent|SetPhysMaterialOverride (Variables|/Game/BluePrints/BP_MoveableRock.BP_MoveableRock_C|GetS_Rounded_Cobble_ullifhwjw_lod3_Var1 _asbp_moveable_rock) "/Game/LightRock.LightRock")
                  (Physics|AddRadialForce (Variables|/Game/BluePrints/BP_MoveableRock.BP_MoveableRock_C|GetS_Rounded_Cobble_ullifhwjw_lod3_Var1 _asbp_moveable_rock) (Variables|Default|GettheLocation) 5e+02 2e+05 "RIF_Constant" false)
                  (Utilities|Platform|CollectGarbage)
                  (Actor|SetLifeSpan 0.4)
                  (Default|DestroyRock _asbp_moveable_rock))))))))))

(fn ConstructionScript)