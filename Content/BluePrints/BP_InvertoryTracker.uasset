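; BP_InvertoryTracker is an inventory counter that tracks how many TR, C and D rocks are held.
; BeginPlay zeroes the three counts, and a separate pickup or sell event for each rock type adds or subtracts one.
; Each change prints the new count to screen as debug output, with no lower bound on selling.
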(event Custom|PickedUp%20TR%20Rock
  (bind _output_get (Variables|Default|SetTR_Amount (+ (Variables|Default|GetTR_Amount) 1)))
  (Development|PrintString (Utilities|String|ToString(Integer) _output_get)))

(event Custom|PickedUP%20%20C%20Rock
  (bind _output_get (Variables|Default|SetC_Amount (+ (Variables|Default|GetC_Amount) 1)))
  (Development|PrintString (Utilities|String|ToString(Integer) _output_get)))

(event Custom|Picked%20Up%20D%20Rock
  (bind _output_get (Variables|Default|SetD_Amount (+ (Variables|Default|GetD_Amount) 1)))
  (Development|PrintString (Utilities|String|ToString(Integer) _output_get)))

(event Custom|Sold%20TR%20Rock
  (bind _output_get (Variables|Default|SetTR_Amount (- (Variables|Default|GetTR_Amount) 1)))
  (Development|PrintString (Utilities|String|ToString(Integer) _output_get)))

(event Custom|Sold%20C%20Rock
  (bind _output_get (Variables|Default|SetC_Amount (- (Variables|Default|GetC_Amount) 1)))
  (Development|PrintString (Utilities|String|ToString(Integer) _output_get)))

(event Custom|Sold%20D%20Rock
  (bind _output_get (Variables|Default|SetD_Amount (- (Variables|Default|GetD_Amount) 1)))
  (Development|PrintString (Utilities|String|ToString(Integer) _output_get)))

(event EventBeginPlay
  (Variables|Default|SetTR_Amount 0)
  (Variables|Default|SetC_Amount 0)
  (Variables|Default|SetD_Amount 0))

(fn ConstructionScript)