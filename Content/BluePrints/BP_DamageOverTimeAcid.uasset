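; BP_DamageOverTimeAcid is an acid hazard that damages actors over time while they overlap its BurnDamage component.
; Overlapping actors with a BP_Health component join ActorsToDamage and are removed when the overlap ends.
; A looping half-second timer applies BaseDamage to every listed actor.
; The overlap shares a branch with AcidShieldActivated, so an active acid shield sets a flag instead of adding the actor.
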(event OnComponentBeginOverlap(BurnDamage)
  (params (OverlappedComponent :type Primitive%20Component%20Object%20Reference) (OtherActor :type Actor%20Object%20Reference) (OtherComp :type Primitive%20Component%20Object%20Reference) (OtherBodyIndex :type Integer) (bFromSweep :type Boolean) (SweepResult :type Hit%20Result%20Structure%20%28by%20ref%29))
  (if (stale Custom|Acid%20Shield%20Activated Acid%20Shield)
    (Variables|Default|SetActivated%20Acid%20Shield true)
    (else
      (Utilities|IsValid (Actor|GetComponentbyClass OtherActor "/Game/BluePrints/BP_Health.BP_Health_C")
        (:Is%20Valid
          (Variables|Default|SetAcid%20Shield%20Status false)
          (Utilities|Array|Add (Variables|Default|GetActorsToDamage) OtherActor))))))

(event OnComponentEndOverlap(BurnDamage)
  (params (OverlappedComponent :type Primitive%20Component%20Object%20Reference) (OtherActor :type Actor%20Object%20Reference) (OtherComp :type Primitive%20Component%20Object%20Reference) (OtherBodyIndex :type Integer))
  (bind _actorstodamage (Variables|Default|GetActorsToDamage))
  (bind _returnvalue (Utilities|Array|FindItem _actorstodamage OtherActor))
  (if (>= _returnvalue 0)
    (Utilities|Array|RemoveIndex (Variables|Default|GetActorsToDamage) _returnvalue)))

(event Custom|DamageTick
  (for _array_element (Variables|Default|GetActorsToDamage)
    (Game|Damage|ApplyDamage _array_element (Variables|Default|GetBase%20Damage) 0 0)))

(event Custom|Acid%20Shield%20Activated
  (params (Acid%20Shield :type Boolean))
  (if Acid%20Shield
    (Variables|Default|SetActivated%20Acid%20Shield true)
    (else
      (Utilities|IsValid (Actor|GetComponentbyClass (stale OnComponentBeginOverlap(BurnDamage) OtherActor) "/Game/BluePrints/BP_Health.BP_Health_C")
        (:Is%20Valid
          (Variables|Default|SetAcid%20Shield%20Status false)
          (Utilities|Array|Add (Variables|Default|GetActorsToDamage) (stale OnComponentBeginOverlap(BurnDamage) OtherActor)))))))

(event EventBeginPlay
  (Utilities|Time|SetTimerbyEvent (delegate Custom|DamageTick) 0.5 true))

(fn ConstructionScript)