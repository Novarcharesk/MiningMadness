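; BP_ScanCollision is a short-lived scan actor whose collision volume changes size over time, then destroys itself.
; On BeginPlay it stores the collider's scale and plays a timeline whose ScanColliderExpand track sets uniform world scale each update, destroying the actor when finished.
; Each actor overlap adds an audio component.
; A disconnected vector-lerp scaling branch from InitialScale is left unused.
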(event EventBeginPlay
  (Variables|Default|SetScan%20Scale (.scale (Transformation|GetRelativeTransform (Variables|Default|GetScanCollision))))
  (bind _scancolliderexpand (Timeline|Timeline PlayFromStart)
    (:Update
      (Transformation|SetWorldScale3D (Variables|Default|GetScanCollision) (Math|Vector|MakeVector _scancolliderexpand _scancolliderexpand _scancolliderexpand)))
    (:Finished
      (Actor|DestroyActor))))

(event Collision|EventActorBeginOverlap
  (params (OtherActor :type Actor%20Object%20Reference))
  (AddComponent|AddAudioComponent false))

(fn ConstructionScript)