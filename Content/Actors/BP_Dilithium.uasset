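; BP_Dilithium is a dilithium actor with a sphere mesh and a timed material reset, apparently tied to scanning.
; BeginPlay fills the BigGemStoneThreeSpawnPoint array with its five spawn points; this graph does not use the array further.
; Tick counts down RemainingScanTime, and below zero it restores the wrinkled-paper material on the sphere and restarts the timer.
; The reset repeats on every cycle, and nothing here applies an alternate material.
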(event EventBeginPlay
  (Variables|Default|SetBig%20Gem%20Stone%20Three%20SpawnPoint (Utilities|Array|MakeArray (Variables|Default|GetSpawnPoint3) (Variables|Default|GetSpawnPoint2) (Variables|Default|GetSpawnPoint1) (Variables|Default|GetSpawnPoint) (Variables|Default|GetSpawnPoint4))))

(event EventTick
  (params (DeltaSeconds :type Float%20%28single-precision%29))
  ;[1 1 1] Material Change Cooldown
  (Variables|Default|SetRemainingScanTime (- (Variables|Default|GetRemainingScanTime) DeltaSeconds))
  (if (< (Variables|Default|GetRemainingScanTime) 0.0)
    (Rendering|Material|SetMaterial (Variables|Default|GetSphere) 0 "/Game/Megascans/Surfaces/Wrinkled_Paper_rm0kg3p0/MI_Wrinkled_Paper_rm0kg3p0_2K.MI_Wrinkled_Paper_rm0kg3p0_2K")
    (Variables|Default|SetRemainingScanTime 3.0)))

(fn ConstructionScript
  (|CallParentFunction))