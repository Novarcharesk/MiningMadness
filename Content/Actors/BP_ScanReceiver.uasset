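; BP_ScanReceiver is a scannable actor, apparently a Chimerium ore chunk, that glows when detected.
; An overlap on its Collider prints a detection message and switches the Sphere to the scan glow material.
; Tick runs a repeating three-second countdown that restores the base material each time it expires.
; Overlaps do not reset that countdown, so the glow's duration varies.
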(event OnComponentBeginOverlap(Collider)
  (params (OverlappedComponent :type Primitive%20Component%20Object%20Reference) (OtherActor :type Actor%20Object%20Reference) (OtherComp :type Primitive%20Component%20Object%20Reference) (OtherBodyIndex :type Integer) (bFromSweep :type Boolean) (SweepResult :type Hit%20Result%20Structure%20%28by%20ref%29))
  (Development|PrintString "A chunk of Chimerium has been detected!")
  (Rendering|Material|SetMaterial (Variables|Default|GetSphere) 0 "/Game/Materials/M_ScanGlow.M_ScanGlow"))

(event EventTick
  (params (DeltaSeconds :type Float%20%28single-precision%29))
  ;[1 1 1] Material Change Cooldown
  (Variables|Default|SetRemainingScanTime (- (Variables|Default|GetRemainingScanTime) DeltaSeconds))
  (if (< (Variables|Default|GetRemainingScanTime) 0.0)
    (Rendering|Material|SetMaterial (Variables|Default|GetSphere) 0 "/Game/FPWeapon/Materials/BaseMaterial.BaseMaterial")
    (Variables|Default|SetRemainingScanTime 3.0)))

(fn ConstructionScript)