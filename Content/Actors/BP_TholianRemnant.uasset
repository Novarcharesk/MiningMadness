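; Tholian remnant actor with a boulder-material sphere and a timed scan cooldown.
; BeginPlay fills BigStoneTwoSpawnPositions with seven SpawnRockTwo references, which this graph does not otherwise use.
; Tick counts down RemainingScanTime, then reapplies the Nordic beach boulder material to the sphere and restarts the three-second timer.
; The construction script only calls its parent.
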(event EventBeginPlay
  (Variables|Default|SetBigStoneTwoSpawnPositions (Utilities|Array|MakeArray (Variables|Default|GetSpawnRockTwo4) (Variables|Default|GetSpawnRockTwo5) (Variables|Default|GetSpawnRockTwo6) (Variables|Default|GetSpawnRockTwo2) (Variables|Default|GetSpawnRockTwo1) (Variables|Default|GetSpawnRockTwo) (Variables|Default|GetSpawnRockTwo3))))

(event EventTick
  (params (DeltaSeconds :type Float%20%28single-precision%29))
  ;[1 1 1] Material Change Cooldown
  (Variables|Default|SetRemainingScanTime (- (Variables|Default|GetRemainingScanTime) DeltaSeconds))
  (if (< (Variables|Default|GetRemainingScanTime) 0.0)
    (Rendering|Material|SetMaterial (Variables|Default|GetSphere) 0 "/Game/Megascans/3D_Assets/Nordic_Beach_Boulder_vcyqebjfa/MI_Nordic_Beach_Boulder_vcyqebjfa_2K.MI_Nordic_Beach_Boulder_vcyqebjfa_2K")
    (Variables|Default|SetRemainingScanTime 3.0)))

(fn ConstructionScript
  (|CallParentFunction))