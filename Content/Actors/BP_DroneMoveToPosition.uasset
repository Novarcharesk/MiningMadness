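; Manager actor that moves the BP_DroneAI drones between following the player and a bomb-planting run at BP_MoveableRock.
; Each Tick it snaps to the player and timeline-lerps each drone toward one of three position components, matching player rotation.
; When the rock allows drones and PressedEToStart is set, it moves to the rock, locks player movement, spawns BP_Bomb after a delay, then restores movement.
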(event Custom|Delayed%20Tick)

(event Custom|CustomEvent)

(event EventBeginPlay
  (bind _outactors (Actor|GetAllActorsOfClass "/Game/Actors/BP_DroneAI.BP_DroneAI_C"))
  (Variables|Default|SetDronesArray _outactors))

(event EventTick
  (params (DeltaSeconds :type Float%20%28single-precision%29))
  (bind _dronesarray (Variables|Default|GetDronesArray))
  (bind _dronesarray_2 (Variables|Default|GetDronesArray))
  (bind _returnvalue (Actor|GetActorOfClass "/Game/BluePrints/BP_MoveableRock.BP_MoveableRock_C"))
  (if (Variables|/Game/BluePrints/BP_MoveableRock.BP_MoveableRock_C|GetcanUseDrone _returnvalue)
    (if (Variables|Default|GetpressedEToStart)
      (bind _returnvalue_2 (Actor|GetActorOfClass "/Game/FirstPerson/Blueprints/BP_FirstPersonCharacter.BP_FirstPersonCharacter_C"))
      (Variables|/Game/FirstPerson/Blueprints/BP_FirstPersonCharacter.BP_FirstPersonCharacter_C|SetCanMove _returnvalue_2 false)
      (Utilities|FlowControl|Sequence
        (:then_0
          (Utilities|Time|SetTimerbyEvent (delegate Custom|Delayed%20Tick) 1.0 true)
          (bind _returnvalue_3 (Actor|GetActorOfClass "/Game/BluePrints/BP_MoveableRock.BP_MoveableRock_C"))
          (Transformation|SetActorLocation (Transformation|GetActorLocation _returnvalue_3) false false)
          (Transformation|SetActorRotation (Math|Rotator|MakeRotator 0.0 0.0 (.yaw (Transformation|GetActorRotation _returnvalue_3))))
          (Utilities|FlowControl|Delay 1.0)
          (Variables|Default|SetBombAmount 0)
          (bind _output_get (Variables|Default|SetBombAmount (+ (Variables|Default|GetBombAmount) (Variables|Default|GetbombMaxAmount))))
          (if (== _output_get 1)
            (Game|SpawnActorfromClass "/Game/BluePrints/BP_Bomb.BP_Bomb_C" (Math|Conversions|ToTransform(Vector) (Transformation|GetWorldLocation (Variables|/Game/BluePrints/BP_MoveableRock.BP_MoveableRock_C|GetBombPlantLocation (stale _returnvalue_5)))) "Undefined" "OverrideRootScale" 0 0)
            (Utilities|FlowControl|Delay 1.0)
            (bind _returnvalue_4 (Actor|GetActorOfClass "/Game/FirstPerson/Blueprints/BP_FirstPersonCharacter.BP_FirstPersonCharacter_C"))
            (Variables|/Game/FirstPerson/Blueprints/BP_FirstPersonCharacter.BP_FirstPersonCharacter_C|SetCanMove _returnvalue_4 true)
            (Variables|Default|SetpressedEToStart false)))
        (:then_1
          (Variables|Default|SetPosition1Transform (Utilities|Array|MakeArray (Transformation|GetWorldLocation (Variables|Default|GetPosition1)) (Transformation|GetWorldLocation (Variables|Default|GetPosition2)) (Transformation|GetWorldLocation (Variables|Default|GetPosition3))))
          (Timeline|ExplosiveDrone Play
            (:Finished
              (for (_array_element _array_index) _dronesarray_2
                _)
              (bind _returnvalue_5 (Actor|GetActorOfClass "/Game/BluePrints/BP_MoveableRock.BP_MoveableRock_C"))
              (Utilities|FlowControl|Sequence
                (:then_0
                  (Transformation|SetActorLocation _array_element (Math|Vector|Lerp(Vector) (Transformation|GetActorLocation (Utilities|Array|Get(acopy) _dronesarray_2 _array_index)) (|MoveableRockLocation _returnvalue_5) 0.0) false false))
                (:then_1
                  (Transformation|SetActorRotation _array_element (Transformation|GetActorRotation (Game|Player|GetPlayerPawn 0)))))))))
      (else
        (Utilities|FlowControl|Sequence :!label _label
          (:then_0
            (Utilities|Time|SetTimerbyEvent (delegate Custom|CustomEvent) 1.0 true)
            (bind _returnvalue_6 (Actor|GetActorOfClass "/Game/FirstPerson/Blueprints/BP_FirstPersonCharacter.BP_FirstPersonCharacter_C"))
            (Transformation|SetActorLocation (Transformation|GetActorLocation _returnvalue_6) false false)
            (Transformation|SetActorRotation (Math|Rotator|MakeRotator 0.0 0.0 (.yaw (Transformation|GetActorRotation _returnvalue_6)))))
          (:then_1
            (Variables|Default|SetPosition1Transform (Utilities|Array|MakeArray (Transformation|GetWorldLocation (Variables|Default|GetPosition1)) (Transformation|GetWorldLocation (Variables|Default|GetPosition2)) (Transformation|GetWorldLocation (Variables|Default|GetPosition3))))
            (bind _dronesfloat (Timeline|Timeline_0 Play)
              (:Update
                (for (_array_element_2 _array_index_2) _dronesarray
                  (Utilities|FlowControl|Sequence
                    (:then_0
                      (Transformation|SetActorLocation _array_element_2 (Math|Vector|Lerp(Vector) (Transformation|GetActorLocation (Utilities|Array|Get(acopy) _dronesarray _array_index_2)) (Utilities|Array|Get(acopy) (Variables|Default|GetPosition1Transform) _array_index_2) _dronesfloat) false false))
                    (:then_1
                      (Transformation|SetActorRotation _array_element_2 (Transformation|GetActorRotation (Game|Player|GetPlayerPawn 0))))))))))))
    (else
      (goto _label))))

(fn ConstructionScript)