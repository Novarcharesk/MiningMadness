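; BP_Chimerium is an actor, apparently a scannable object, with a sphere mesh and a set of gemstone spawn pads.
; On BeginPlay it gathers eight SpawnPad references into GemStoneOneSpawnPoints, which this graph does not use further.
; Tick counts down RemainingScanTime as a material-change cooldown, setting the sphere to a polystyrene material and restarting the timer whenever it drops below zero.
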(event EventTick
  (params (DeltaSeconds :type Float%20%28single-precision%29))
  ;[1 1 1] Material Change Cooldown
  (Variables|Default|SetRemainingScanTime (- (Variables|Default|GetRemainingScanTime) DeltaSeconds))
  (if (< (Variables|Default|GetRemainingScanTime) 0.0)
    (Rendering|Material|SetMaterial (Variables|Default|GetSphere) 0 "/Game/Megascans/Surfaces/Polystyrene_rfya3fp0/MI_Polystyrene_rfya3fp0_2K.MI_Polystyrene_rfya3fp0_2K")
    (Variables|Default|SetRemainingScanTime 3.0)))

(event EventBeginPlay
  (Variables|Default|SetGem%20Stone%20One%20Spawn%20Points (Utilities|Array|MakeArray (Variables|Default|GetSpawnPad) (Variables|Default|GetSpawnPad1) (Variables|Default|GetSpawnPad2) (Variables|Default|GetSpawnPad3) (Variables|Default|GetSpawnPad4) (Variables|Default|GetSpawnPad5) (Variables|Default|GetSpawnPad6) (Variables|Default|GetSpawnPad7))))

(fn ConstructionScript
  (|CallParentFunction))